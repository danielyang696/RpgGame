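; Actor component that handles bow equipping and aiming input for BP_ThirdPersonCharacter, caching its owner on BeginPlay with one delayed retry.
; IA_EquipBow toggles the bow in hand if the character has one, switching movement between controller-facing and movement-oriented rotation.
; While equipped, holding IA_BowShoot sets the aiming flag and shows a crosshair widget, and releasing clears both.
; No arrow firing happens here.
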(event `self.ReceiveBeginPlay`
  (bind _returnvalue (`self.GetOwner`))
  ; Initialize
  (bind _asbp_third_person_character (cast `/Game/ThirdPerson/Blueprints/BP_ThirdPersonCharacter` _returnvalue)
    (:`then`
      (set `self.CharacterBP` _asbp_third_person_character))
    (:`CastFailed`
      (`KismetSystemLibrary.Delay` 0.1)
      (bind _asbp_third_person_character_2 (cast `/Game/ThirdPerson/Blueprints/BP_ThirdPersonCharacter` _returnvalue))
      (set `self.CharacterBP` _asbp_third_person_character_2))))

(event `EnhancedInput|/Game/Input/Actions/IA_BowShoot`
  (params (ActionValue :type Boolean) (ElapsedSeconds :type "Float (double-precision)") (TriggeredSeconds :type "Float (double-precision)") (InputAction :type "InputAction Object Reference" :default "/Game/Input/Actions/IA_BowShoot.IA_BowShoot"))
  ; Bow
  (:`Started`
    (if (`/Game/ThirdPerson/Blueprints/BP_ThirdPersonCharacter.isEquipBow` (`self.characterBP`))
      (set `/Game/ThirdPerson/Blueprints/BP_ThirdPersonCharacter.isAimingWithBow` true (`self.characterBP`))
      (bind _returnvalue (`|CreateWidget` "/Game/UI/WB_Bow_Crosshair.WB_Bow_Crosshair_C"))
      (bind _output_get (set `self.bowCrossHair` _returnvalue))
      (`UserWidget.AddToViewport` _output_get 0)))
  (:`Completed`
    (if (`/Game/ThirdPerson/Blueprints/BP_ThirdPersonCharacter.isEquipBow` (`self.characterBP`))
      (set `/Game/ThirdPerson/Blueprints/BP_ThirdPersonCharacter.isAimingWithBow` false (`self.characterBP`))
      (bind _bowcrosshair (`self.bowCrossHair`)
        (:`then`
          (`Widget.RemoveFromParent` _bowcrosshair)
          (set `self.bowCrossHair` null))
        (:`else`)))))

(event `EnhancedInput|/Game/Input/Actions/IA_EquipBow`
  (params (ActionValue :type Boolean) (ElapsedSeconds :type "Float (double-precision)") (TriggeredSeconds :type "Float (double-precision)") (InputAction :type "InputAction Object Reference" :default "/Game/Input/Actions/IA_EquipBow.IA_EquipBow"))
  (bind _characterbp (`self.characterBP`))
  (bind _characterbp_2 (`self.characterBP`))
  (bind _charactermovement (`Character.CharacterMovement` _characterbp))
  ; Bow
  (:`Started`
    (if (`/Game/ThirdPerson/Blueprints/BP_ThirdPersonCharacter.hasBow` (`self.characterBP`))
      (if (not (`/Game/ThirdPerson/Blueprints/BP_ThirdPersonCharacter.isEquipBow` (`self.characterBP`)))
        (set `/Game/ThirdPerson/Blueprints/BP_ThirdPersonCharacter.isEquipBow` true _characterbp_2)
        (`/Game/ThirdPerson/Blueprints/BP_ThirdPersonCharacter.EquipBowInHand` _characterbp)
        (set `CharacterMovementComponent.bUseControllerDesiredRotation` true _charactermovement)
        (set `CharacterMovementComponent.bOrientRotationToMovement` false _charactermovement)
        (else
          (set `/Game/ThirdPerson/Blueprints/BP_ThirdPersonCharacter.isEquipBow` false _characterbp_2)
          (`/Game/ThirdPerson/Blueprints/BP_ThirdPersonCharacter.UnEquipBowInHand` _characterbp)
          (set `CharacterMovementComponent.bUseControllerDesiredRotation` false _charactermovement)
          (set `CharacterMovementComponent.bOrientRotationToMovement` true _charactermovement))))))