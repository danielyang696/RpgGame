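; BP_Switch is a switch actor that fires when the player character enters its DetectRadius.
; It creates a dynamic material on its Cube at BeginPlay.
; Overlap by BP_ThirdPersonCharacter turns the cube's Color parameter green and sends BridgeActivateMessage to the referenced ActorToActivate.
; Leaving the radius does nothing, as the logic that sets the color to red is disconnected.
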(event `self.ReceiveBeginPlay`
  (bind _returnvalue (`PrimitiveComponent.CreateDynamicMaterialInstance` (`self.Cube`) 0 null "None"))
  (set `self.DynamicMat` _returnvalue))

(event `self.Detect Radius.OnComponentBeginOverlap`
  (params (OverlappedComponent :type "PrimitiveComponent Object Reference") (OtherActor :type "Actor Object Reference") (OtherComp :type "PrimitiveComponent Object Reference") (OtherBodyIndex :type Integer) (bFromSweep :type Boolean) (SweepResult :type "HitResult Structure (by ref)"))
  (cast `/Game/ThirdPerson/Blueprints/BP_ThirdPersonCharacter` OtherActor)
  (`MaterialInstanceDynamic.SetVectorParameterValue` (`self.DynamicMat`) "Color" (struct :`G` 1.0 :`A` 1.0))
  (message `/Game/Buleprints/Remiu/BPI_Bridge_Activate.Bridge Activate` (`self.Actor To Activate`)))

(event `self.Detect Radius.OnComponentEndOverlap`
  (params (OverlappedComponent :type "PrimitiveComponent Object Reference") (OtherActor :type "Actor Object Reference") (OtherComp :type "PrimitiveComponent Object Reference") (OtherBodyIndex :type Integer)))

(fn `UserConstructionScript`)