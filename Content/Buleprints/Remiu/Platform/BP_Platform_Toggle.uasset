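; Platform actor that toggles between its BeginPlay location and a TargetActor's location on each BridgeActivate call.
; BridgeActivate flips IsAtTarget and passes the current and destination locations to MoveTo, which lerps the actor via a forward or backward Timeline, chosen by comparing those locations.
; Its DoOnce resets right after MoveTo is called, so it does not lock out calls during movement.
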(event `self.ReceiveBeginPlay`
  (set `self.StartLocation` (`self.K2_GetActorLocation`)))

(event `/Game/Buleprints/Remiu/BPI_Bridge_Activate.Bridge Activate`
  (bind _returnvalue (`self.K2_GetActorLocation`))
  (`/Engine/EditorBlueprintResources/StandardMacros.DoOnce` false :!label _label
    (:`Completed`
      (if (`self.bIsAtTarget`)
        (`self.MoveTo` (`self.StartLocation`) _returnvalue)
        (set `self.bIsAtTarget` false)
        (goto _label :!via `Reset`)
        (else
          (`self.MoveTo` (`self.K2_GetActorLocation` (`self.TargetActor`)) _returnvalue)
          (set `self.bIsAtTarget` true)
          (goto _label :!via `Reset`))))))

(event `/Game/Buleprints/Remiu/Platform/BPI_Platform_MoveTo.MoveTo`
  (params (TargetLocation :type "Vector Structure") (StartLocation :type "Vector Structure"))
  (if (== TargetLocation (`self.StartLocation`))
    (bind (_direction _alpha) (`Timeline|Timeline_Backward` :!via `PlayFromStart`)
      (:`Update`
        (`self.K2_SetActorLocation` (`KismetMathLibrary.VLerp` TargetLocation StartLocation _alpha))))
    (else
      (bind (_direction_2 _alpha_2) (`Timeline|Timeline_Forward` :!via `PlayFromStart`)
        (:`Update`
          (`self.K2_SetActorLocation` (`KismetMathLibrary.VLerp` StartLocation TargetLocation _alpha_2)))))))

(fn `UserConstructionScript`)