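; BPC_Interact is an interaction component that lets its owning actor interact with nearby objects.
; When IA_Interact starts and CanInteract is true, it runs a sphere trace on the Visibility channel from the owner's location.
; The trace end is offset by the owner's scaled rotation rather than an explicit forward vector.
; InteractMessage is sent to the hit actor without checking whether the trace hit.
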(event `EnhancedInput|/Game/Input/Actions/IA_Interact`
  (params (ActionValue :type Boolean) (ElapsedSeconds :type "Float (double-precision)") (TriggeredSeconds :type "Float (double-precision)") (InputAction :type "InputAction Object Reference" :default "/Game/Input/Actions/IA_Interact.IA_Interact"))
  (bind _returnvalue (`self.GetOwner`))
  (bind _returnvalue_2 (`Actor.K2_GetActorLocation` _returnvalue))
  (:`Started`
    (if (`self.Can Interact`)
      (bind _outhit (`KismetSystemLibrary.SphereTraceSingle` _returnvalue_2 (+ _returnvalue_2 (* (`Actor.K2_GetActorRotation` _returnvalue) 50.0)) 50.0 "TraceTypeQuery1"))
      (if true
        (message `/Game/Buleprints/Remiu/BPI_Interact.Interact` (`.HitActor` (`GameplayStatics.BreakHitResult` _outhit)))))))