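; Player stamina component that holds a current stamina value and exposes functions to spend and restore it.
; DecreaseStamina subtracts a cost only while stamina is above zero and returns true when it is depleted, without clamping values that drop below zero.
; IncreaseStamina adds an amount and caps the result at MaxStamina.
; The event graph has no logic, so all changes depend on external calls.
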(event `self.ReceiveBeginPlay`)

(fn `DecreaseStamina`
  (params (staminaCost :type "Float (double-precision)"))
  (returns (notStaminaLeft :type Boolean))
  (if (not (<= (`self.currentStamina`) 0.0))
    (set `self.currentStamina` (- (`self.currentStamina`) staminaCost)))
  (if (<= (`self.currentStamina`) 0.0)
    (return true)
    (else
      (return false))))

(fn `IncreaseStamina`
  (params (addedStamina :type "Float (double-precision)"))
  (set `self.currentStamina` (+ (`self.currentStamina`) addedStamina))
  (if (> (`self.currentStamina`) (`self.maxStamina`))
    (set `self.currentStamina` (`self.maxStamina`))))