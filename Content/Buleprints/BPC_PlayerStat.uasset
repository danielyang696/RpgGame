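; Actor component that holds health and stamina for the player, AI and dummy characters and updates their progress bars.
; On BeginPlay, after a one-tick delay, it casts its owner to set the character type, which selects the HUD or overhead health bar.
; Decrease functions report depletion and increase functions clamp to the maximum.
; Stamina functions and IncreaseHealth write only to the player's HUD.
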(event `self.ReceiveBeginPlay`
  (`KismetSystemLibrary.DelayUntilNextTick`)
  (bind _asbp_third_person_character (cast `/Game/ThirdPerson/Blueprints/BP_ThirdPersonCharacter` (`self.GetOwner`))
    (:`then`
      (set `self.CharacterBP` _asbp_third_person_character)
      (set `self.characterType` "NewEnumerator0")
      (set `self.isPlayer` true))
    (:`CastFailed`
      (bind _asbp_dummy (cast `/Game/Buleprints/BP_Dummy` (`self.GetOwner`))
        (:`then`
          (set `self.BP_Dummy` _asbp_dummy)
          (set `self.characterType` "NewEnumerator2"))
        (:`CastFailed`
          (bind _asbp_ai (cast `/Game/AI/BP_AI` (`self.GetOwner`)))
          (set `self.BP AI` _asbp_ai)
          (set `self.characterType` "NewEnumerator1")))
      (set `self.isPlayer` false)))
  (`ProgressBar.SetPercent` (select `/Game/Buleprints/E_CharacterType` (`self.characterType`) :`NewEnumerator0` (`/Game/UI/WB_HUD.HealthBar` (`/Game/ThirdPerson/Blueprints/BP_ThirdPersonCharacter.HUD` (`self.CharacterBP`))) :`NewEnumerator1` (`/Game/UI/WB_DummyHealthBar.HealthBar` (`/Game/AI/BP_AI.HealthBarUI` (`self.BP AI`))) :`NewEnumerator2` (`/Game/UI/WB_DummyHealthBar.HealthBar` (`/Game/Buleprints/BP_Dummy.HealthBarUI` (`self.BP_Dummy`)))) (/ (`self.currentHealth`) (`self.maxHealth`)))
  (if (`self.isPlayer`)
    (`ProgressBar.SetPercent` (`/Game/UI/WB_HUD.StaminaBar` (`/Game/ThirdPerson/Blueprints/BP_ThirdPersonCharacter.HUD` (`self.CharacterBP`))) (/ (`self.currentStamina`) (`self.maxStamina`)))))

(fn `DecreaseHealth`
  (params (damage :type "Float (double-precision)"))
  (returns (isPlayerDie :type Boolean))
  (if (not (<= (`self.currentHealth`) 0.0))
    (bind _output_get (set `self.currentHealth` (- (`self.currentHealth`) damage)))
    (`ProgressBar.SetPercent` (select `/Game/Buleprints/E_CharacterType` (`self.characterType`) :`NewEnumerator0` (`/Game/UI/WB_HUD.HealthBar` (`/Game/ThirdPerson/Blueprints/BP_ThirdPersonCharacter.HUD` (`self.CharacterBP`))) :`NewEnumerator1` (`/Game/UI/WB_DummyHealthBar.HealthBar` (`/Game/AI/BP_AI.HealthBarUI` (`self.BP AI`))) :`NewEnumerator2` (`/Game/UI/WB_DummyHealthBar.HealthBar` (`/Game/Buleprints/BP_Dummy.HealthBarUI` (`self.BP_Dummy`)))) (/ _output_get (`self.maxHealth`)))
    (if (<= (`self.currentHealth`) 0.0)
      _
      (else
        (return false))))
  (return true))

(fn `DecreaseStamina`
  (params (staminaCost :type "Float (double-precision)"))
  (returns (notStaminaLeft :type Boolean))
  (if (not (<= (`self.currentStamina`) 0.0))
    (bind _output_get (set `self.currentStamina` (- (`self.currentStamina`) staminaCost)))
    (`ProgressBar.SetPercent` (`/Game/UI/WB_HUD.StaminaBar` (`/Game/ThirdPerson/Blueprints/BP_ThirdPersonCharacter.HUD` (`self.CharacterBP`))) (/ _output_get (`self.maxStamina`))))
  (if (<= (`self.currentStamina`) 0.0)
    (return true)
    (else
      (return false))))

(fn `IncreaseHealth`
  (params (addedHealth :type "Float (double-precision)"))
  (set `self.currentHealth` (+ (`self.currentHealth`) addedHealth))
  (if (> (`self.currentHealth`) (`self.maxHealth`))
    (bind _output_get (set `self.currentHealth` (`self.maxHealth`))))
  (`ProgressBar.SetPercent` (`/Game/UI/WB_HUD.HealthBar` (`/Game/ThirdPerson/Blueprints/BP_ThirdPersonCharacter.HUD` (`self.CharacterBP`))) (/ _output_get (`self.maxHealth`))))

(fn `IncreaseStamina`
  (params (addedStamina :type "Float (double-precision)"))
  (set `self.currentStamina` (+ (`self.currentStamina`) addedStamina))
  (if (> (`self.currentStamina`) (`self.maxStamina`))
    (bind _output_get (set `self.currentStamina` (`self.maxStamina`))))
  (`ProgressBar.SetPercent` (`/Game/UI/WB_HUD.StaminaBar` (`/Game/ThirdPerson/Blueprints/BP_ThirdPersonCharacter.HUD` (`self.CharacterBP`))) (/ _output_get (`self.maxStamina`))))