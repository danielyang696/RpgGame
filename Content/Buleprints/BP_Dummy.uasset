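; Dummy enemy character that takes hits, shows a health bar turned toward the player camera, and ragdolls on death.
; AnyDamage plays a random hit montage, knocks it along the player's forward vector, and reduces health through BPCPlayerStat.
; When DecreaseHealth returns true, it ragdolls, plays a death sound, hides the bar, disables capsule collision and removes its first tag.
; BackFatal plays a fatal-hit montage with delayed ragdoll and sound, returning a reference location and yaw-offset rotation.
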(event `self.ReceiveBeginPlay`
  (bind _aswb_dummy_health_bar (cast `/Game/UI/WB_DummyHealthBar` (`WidgetComponent.GetWidget` (`self.Health Bar Widget`))))
  (set `self.HealthBarUI` _aswb_dummy_health_bar))

(event `self.ReceiveTick`
  (params (DeltaSeconds :type "Float (single-precision)"))
  (`SceneComponent.K2_SetWorldRotation` (`self.Health Bar Widget`) (`KismetMathLibrary.FindLookAtRotation` (`SceneComponent.K2_GetComponentLocation` (`self.Health Bar Widget`)) (`SceneComponent.K2_GetComponentLocation` (`PlayerCameraManager.TransformComponent` (`GameplayStatics.GetPlayerCameraManager` 0)))) false false))

(event `Ragdoll`
  ; Ragdoll (enable simulate physics when target die
  (`|ExecutionSequence`
    (:`then_0`
      (`KismetSystemLibrary.Delay` 2.8)
      (`PrimitiveComponent.SetSimulatePhysics` (`self.Mesh`) true))
    (:`then_1`
      (`KismetSystemLibrary.Delay` 1.0)
      (`GameplayStatics.PlaySoundAtLocation` "/Game/Audio/Grunt/SC_Death.SC_Death" (`self.K2_GetActorLocation`) (struct) 1.0 1.0 0.0 null null null null))))

(event `self.ReceiveAnyDamage`
  (params (Damage :type "Float (single-precision)") (DamageType :type "DamageType Object Reference") (InstigatedBy :type "Controller Object Reference") (DamageCauser :type "Actor Object Reference"))
  (`self.PlayAnimMontage` (`|GetArrayItem` (`self.Hit_AnimMontage`) (`KismetMathLibrary.RandomIntegerInRange` 0 (- (`KismetArrayLibrary.Array_Length` (`self.Hit_AnimMontage`)) 1))))
  (bind _asbp_third_person_character (cast `/Game/ThirdPerson/Blueprints/BP_ThirdPersonCharacter` (`GameplayStatics.GetPlayerCharacter` 0)))
  (`CharacterMovementComponent.AddImpulse` (`self.CharacterMovement`) (* (`KismetMathLibrary.GetForwardVector` (`self.K2_GetActorRotation` _asbp_third_person_character)) 2000.0) true)
  (bind _isplayerdie (`/Game/Buleprints/BPC_PlayerStat.DecreaseHealth` (`self.BPC_PlayerStat`) Damage))
  (if _isplayerdie
    (`KismetSystemLibrary.Delay` 0.2)
    (`PrimitiveComponent.SetSimulatePhysics` (`self.Mesh`) true)
    (`GameplayStatics.PlaySoundAtLocation` "/Game/Audio/Grunt/SC_Death.SC_Death" (`self.K2_GetActorLocation`) (struct) 1.0 1.0 0.0 null null null null)
    (`SceneComponent.SetVisibility` (`self.Health Bar Widget`) false false)
    (`PrimitiveComponent.SetCollisionEnabled` (`self.CapsuleComponent`) "NoCollision")
    (`KismetArrayLibrary.Array_Remove` (`self.Tags`))))

(fn `BackFatal`
  (returns (refLocation :type "Vector Structure") (fatalRotation :type "Rotator Structure"))
  (`self.PlayAnimMontage` "/Game/Characters/RpgGame/Animation/Fatal/AS_OneHand_Up_Fatal_Hit_1_Montage.AS_OneHand_Up_Fatal_Hit_1_Montage")
  (`self.Ragdoll`)
  (return (`SceneComponent.K2_GetComponentLocation` (`self.ref location`)) (`KismetMathLibrary.MakeRotator` (.roll (`self.K2_GetActorRotation`)) (.pitch (`self.K2_GetActorRotation`)) (+ (.yaw (`self.K2_GetActorRotation`)) 30.0))))

(fn `UserConstructionScript`)