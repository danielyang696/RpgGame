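; Combat component that runs a character's melee attacks: ground smash, short-range swing, long-range leap and front/back fatal executions.
; Montage notifies trigger AOE actor spawns, arc-solved launches toward the target and timer-looped sword sphere traces, reporting attack end to the owner through interface messages.
; Sword hits damage each non-team actor once per swing, report parries and add brief time-dilation hit-stop.
; Fatal attacks use motion warping, timed damage and camera shakes.
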(event `FatalAttack`
  (params (attackTatget :type "Actor Object Reference") (MeshComponent :type "SkeletalMeshComponent Object Reference") (MotionWarpingComponent :type "MotionWarpingComponent Object Reference") (FatalType :type "/Game/Buleprints/EnumAndStructure/E_FatalType Enum" :default "NewEnumerator0"))
  (bind _returnvalue (`self.GetOwner`))
  (bind _returnvalue_2 (`Actor.K2_GetActorLocation` (`self.GetOwner` MeshComponent)))
  ; Fatal Attack
  (`|ExecutionSequence`
    (:`then_0`
      (bind (_reflocation _fatalrotation) (message `/Game/Buleprints/BPI_Fatal.Fatal` attackTatget FatalType))
      (bind _damageinfo (`self.Play Fatal Anim` MeshComponent FatalType)
        (:`OnCompleted`
          ;; delay是為了等敵人的被處決動畫撥放完成
          (if (stale _wasdamaged)
            (`KismetSystemLibrary.Delay` 1.84)
            (`AISense_Damage.ReportDamageEvent` attackTatget _returnvalue 120.0 (`Actor.K2_GetActorLocation` _returnvalue))))
        (:`then`
          (`MotionWarpingComponent.AddOrUpdateWarpTarget` MotionWarpingComponent (make `MotionWarpingTarget` "FatalWarp" _reflocation _fatalrotation))
          (`KismetSystemLibrary.Delay` 0.89)
          (bind _wasdamaged (message `/Game/Damage_System/BPI_Damagable.TakeDamage` attackTatget _damageinfo)))))
    (:`then_1`
      (`KismetSystemLibrary.Delay` 0.85)
      (`GameplayStatics.PlayWorldCameraShake` "/Game/Buleprints/BP_CameraShake.BP_CameraShake_C" _returnvalue_2 0.0 2000.0)
      (`KismetSystemLibrary.Delay` 1.6)
      (`GameplayStatics.PlayWorldCameraShake` "/Game/Buleprints/BP_CameraShake.BP_CameraShake_C" _returnvalue_2 0.0 1000.0))))

(event `GroundSmash`
  (params (AttackInfo :type "/Game/Buleprints/EnumAndStructure/S_AttackInfo Structure") (Radius :type "Float (single-precision)"))
  (bind (_attacktarget _montage _damageinfo) (break `/Game/Buleprints/EnumAndStructure/S_AttackInfo` AttackInfo))
  (bind _returnvalue (`self.GetOwner`))
  ; Attack
  (bind _mesh (`self.AttackBase` _attacktarget))
  (bind _notifyname (`|PlayMontage` _mesh _montage 1.0 0.0 "None" false)
    (:`then`
      (message `/Game/Damage_System/BPI_Damagable.SetIsInterrutible` _returnvalue false))
    (:`OnCompleted`
      (message `/Game/Enemy/New_Base_AI/AI/BPI_EnemyAI.AttackEnd` _returnvalue _attacktarget :!label _label))
    (:`OnInterrupted`
      (goto _label))
    (:`OnNotifyBegin`
      (switch `name` _notifyname
        (:`AOE`
          (`self.AOEDamage` Radius _damageinfo))
        (:`CanMove`
          (message `/Game/Damage_System/BPI_Damagable.SetIsInterrutible` _returnvalue true))))))

(event `Jump To AttackTarget`
  (params (AttackTarget :type "Actor Object Reference"))
  ; Jump To Target
  (bind _returnvalue (`self.Calculate Futrue Actor Location` AttackTarget))
  (bind _outlaunchvelocity (`GameplayStatics.SuggestProjectileVelocity_CustomArc` (`Actor.K2_GetActorLocation` (`self.GetOwner`)) (`KismetMathLibrary.MakeVector` (.x _returnvalue) (.y _returnvalue) (.z _returnvalue)) 0.0 0.95))
  (`Character.LaunchCharacter` (cast `Character` (`self.GetOwner`) :!pure true) _outlaunchvelocity false true))

(event `Short Range Attack`
  (params (AttackInfo :type "/Game/Buleprints/EnumAndStructure/S_AttackInfo Structure") (`Trace Radius` :type "Float (double-precision)") (SwordButtom :type "ArrowComponent Object Reference") (SwordTop :type "ArrowComponent Object Reference"))
  (bind (_attacktarget _montage _damageinfo) (break `/Game/Buleprints/EnumAndStructure/S_AttackInfo` AttackInfo))
  ; Attack
  (bind _mesh (`self.AttackBase` _attacktarget))
  (bind _notifyname (`|PlayMontage` _mesh _montage 1.0 0.0 "None" false)
    (:`OnCompleted`
      (message `/Game/Enemy/New_Base_AI/AI/BPI_EnemyAI.AttackEnd` (`self.GetOwner`) _attacktarget :!label _label_2))
    (:`OnInterrupted`
      (goto _label_2))
    (:`OnNotifyBegin`
      (switch `name` _notifyname
        (:`Trace`
          (`self.Sword Trace Start` SwordButtom SwordTop _damageinfo `Trace Radius`))))
    (:`OnNotifyEnd`
      (switch `name` _notifyname
        (:`Trace`
          (`self.Sword Trace End`))))))

(event `Sword Trace Start`
  (params (SwordButtom :type "ArrowComponent Object Reference") (SwordTop :type "ArrowComponent Object Reference") (DamageInfo :type "/Game/Damage_System/S_DamageInfo Structure") (Radius :type "Float (single-precision)"))
  ; Sword Trace
  (`KismetArrayLibrary.Array_Clear` (`self.ActorAlreadyDamaged`))
  (bind _returnvalue (`KismetSystemLibrary.K2_SetTimerDelegate` (delegate `Sword Trace Loop`) 0.01 true))
  (set `self.SwordTraceLoop` _returnvalue))

(event `Sword Trace Loop`
  (bind _returnvalue (`self.GetOwner`))
  ; Sword Trace
  (bind (_outhits _returnvalue_2) (`KismetSystemLibrary.SphereTraceMultiForObjects` (`SceneComponent.K2_GetComponentLocation` (stale `Sword Trace Start` SwordButtom)) (`SceneComponent.K2_GetComponentLocation` (stale `Sword Trace Start` SwordTop)) (stale `Sword Trace Start` Radius) (`|MakeArray` "ObjectTypeQuery3" :!type "EObjectTypeQuery Enum")))
  (if _returnvalue_2
    (bind (_actor_damaged _was_damaged) (`self.Damage All Non Team Meber` _outhits (stale `Sword Trace Start` DamageInfo)))
    (if _was_damaged
      (`/Engine/EditorBlueprintResources/StandardMacros.DoOnce` false :!label _label_3
        (:`Completed`
          (set `Actor.CustomTimeDilation` 0.05 _returnvalue)
          (`KismetSystemLibrary.Delay` 0.05)
          (set `Actor.CustomTimeDilation` 1.0 _returnvalue)
          (`self.Play Hit Audio`))))))

(event `AOEDamage`
  (params (Radius :type "Float (single-precision)") (DamageInfo :type "/Game/Damage_System/S_DamageInfo Structure"))
  (bind _returnvalue (`self.GetOwner`))
  ; Sword Trace
  (bind _returnvalue_2 (`|SpawnActorFromClass` "/Game/AOE/BP_AOE_Base.BP_AOE_Base_C" (`KismetMathLibrary.MakeTransform` (+ (`Actor.K2_GetActorLocation` _returnvalue) (* (`Actor.GetActorForwardVector` _returnvalue) 170.0))) "Undefined" "MultiplyWithRoot" null (cast `Pawn` (`self.GetOwner`) :!pure true)))
  (set `/Game/AOE/BP_AOE_Base.Radius` Radius _returnvalue_2)
  (add `/Game/AOE/BP_AOE_Base.OnAOEOverlapActors` _returnvalue_2 (delegate `AOEDamageActor`))
  (`/Game/AOE/BP_AOE_Base.Trigger` _returnvalue_2))

(event `AOEDamageActor`
  (params (Actor :type "Actor Object Reference"))
  ; Sword Trace
  (message `/Game/Damage_System/BPI_Damagable.TakeDamage` Actor (stale `AOEDamage` DamageInfo)))

(event `Long Range Jump Attack`
  (params (AttackInfo :type "/Game/Buleprints/EnumAndStructure/S_AttackInfo Structure") (`Trace Radius` :type "Float (single-precision)") (SwordButtom :type "ArrowComponent Object Reference") (SwordTop :type "ArrowComponent Object Reference"))
  (bind (_attacktarget _montage _damageinfo) (break `/Game/Buleprints/EnumAndStructure/S_AttackInfo` AttackInfo))
  (bind _returnvalue (`self.GetOwner`))
  (bind _returnvalue_2 (`self.GetOwner`))
  (bind (_returnvalue_x _returnvalue_y) (`KismetMathLibrary.BreakVector` (`Actor.GetActorForwardVector` _returnvalue_2)))
  ; Attack
  (bind _mesh (`self.AttackBase` _attacktarget))
  (bind _notifyname (`|PlayMontage` _mesh _montage 1.0 0.0 "None" false)
    (:`then`
      (message `/Game/Damage_System/BPI_Damagable.SetIsInterrutible` _returnvalue false))
    (:`OnCompleted`
      (message `/Game/Enemy/New_Base_AI/AI/BPI_EnemyAI.AttackEnd` _returnvalue _attacktarget :!label _label_4))
    (:`OnInterrupted`
      (goto _label_4))
    (:`OnNotifyBegin`
      (switch `name` _notifyname
        (:`Jump`
          ;; 先往上跳
          (`Character.LaunchCharacter` (cast `Character` _returnvalue_2 :!pure true) (`KismetMathLibrary.MakeVector` (* _returnvalue_x 400.0) (* _returnvalue_y 400.0) 700.0) false true))
        (:`Second Jump`
          (`self.Jump To AttackTarget` _attacktarget))
        (:`Trace`
          (`self.Sword Trace Start` SwordButtom SwordTop _damageinfo `Trace Radius`))
        (:`CanMove`
          (message `/Game/Damage_System/BPI_Damagable.SetIsInterrutible` _returnvalue true))))
    (:`OnNotifyEnd`
      (switch `name` _notifyname
        (:`Trace`
          (`self.Sword Trace End`))))))

(event `Sword Trace End`
  ; Sword Trace
  (`KismetSystemLibrary.K2_ClearAndInvalidateTimerHandle` (`self.SwordTraceLoop`))
  (goto _label_3 :!via `Reset`))

(event `Play Hit Audio`
  ; Hit Audio
  (`GameplayStatics.PlaySoundAtLocation` "/Game/Audio/Hit/sword_slash.sword_slash" (`Actor.K2_GetActorLocation` (`self.GetOwner`)) (struct) 1.0 (`KismetMathLibrary.RandomFloatInRange` 0.8 1.2) 0.0 "/Game/Audio/SA_Character.SA_Character" null null null))

(fn `AttackBase`
  (params (AttackTarget :type "Actor Object Reference"))
  (returns (Mesh :type "SkeletalMeshComponent Object Reference"))
  (bind _returnvalue (`self.GetOwner`))
  (message `/Game/Enemy/New_Base_AI/AI/BPI_EnemyAI.DefaultAttack` _returnvalue AttackTarget)
  (bind _ascharacter (cast `Character` _returnvalue))
  (return (`Character.Mesh` _ascharacter)))

(fn `Calculate Futrue Actor Location`
  (params (TargetActor :type "Actor Object Reference") (Time :type "Float (double-precision)"))
  (returns (ReturnValue :type "Vector Structure"))
  (bind _returnvalue (`Actor.K2_GetActorLocation` TargetActor))
  (if (== Time 0.0)
    (return _returnvalue)
    (else
      (return (+ _returnvalue (* (* (`Actor.GetVelocity` TargetActor) (1.0 1.0 0.0)) Time))))))

(fn `Check Can Fatal Attack`
  (params (CharacterBP :type "Actor Object Reference"))
  (returns (`Array Element` :type "Actor Object Reference") (canFatalAttack :type Boolean))
  (locals (tempCanFatalAttack :type Boolean))
  ; CheckCanFatalAttack
  (set `local.tempCanFatalAttack` false)
  (for _array_element (`Actor.GetOverlappingActors` CharacterBP null)
    (bind _sameteam (`self.CheckOnSameTeam` _array_element))
    (if (and (not _sameteam) (`KismetSystemLibrary.DoesImplementInterface` _array_element "/Game/Buleprints/BPI_Fatal.BPI_Fatal_C") (`Actor.ActorHasTag` _array_element "Damageable"))
      (set `local.tempCanFatalAttack` true)))
  (return _array_element (`local.tempCanFatalAttack`)))

(fn `CheckOnSameTeam`
  (params (`Hit actor` :type "Object Object Reference"))
  (returns (SameTeam :type Boolean))
  (bind _teamnumber (message `/Game/Damage_System/BPI_Damagable.GetTeamNumber` `Hit actor`))
  (bind _teamnumber_2 (message `/Game/Damage_System/BPI_Damagable.GetTeamNumber` (`self.GetOwner`)))
  (return (== _teamnumber_2 _teamnumber)))

(fn `Damage All Non Team Meber`
  (params (Hits :type "Array of HitResult Structure") (DamageInfo :type "/Game/Damage_System/S_DamageInfo Structure"))
  (returns (`Actor Damaged` :type "Array of Actor Object Reference") (`Was Damaged` :type Boolean))
  (locals (ActorAlreadyDame :type "Array of Actor Object Reference"))
  (for _array_element Hits
    (bind (_bblockinghit _binitialoverlap _time _distance _location _impactpoint _normal _impactnormal _physmat _hitactor) (`GameplayStatics.BreakHitResult` _array_element))
    (if (`Actor.ActorHasTag` _hitactor "Damageable")
      (bind _sameteam (`self.CheckOnSameTeam` _hitactor))
      (if (and (not _sameteam) (not (`KismetArrayLibrary.Array_Contains` (`self.ActorAlreadyDamaged`) _hitactor)))
        (`KismetArrayLibrary.Array_AddUnique` (`self.ActorAlreadyDamaged`) _hitactor)
        (bind (_wasdamaged _parrysucces) (message `/Game/Damage_System/BPI_Damagable.TakeDamage` _hitactor DamageInfo))
        (if _wasdamaged
          (`GameplayStatics.SpawnEmitterAtLocation` "/Game/FX_Blood/Particles/Blood/P_Blood_Splat_Cone.P_Blood_Splat_Cone" _location (`KismetMathLibrary.MakeRotFromXY` _normal _normal) (1.0 1.0 1.0) true "AutoRelease")
          (else
            ; Handle Parry
            (if _parrysucces
              (`self.OnBeParried`)))))))
  (return (`self.ActorAlreadyDamaged`) _wasdamaged))