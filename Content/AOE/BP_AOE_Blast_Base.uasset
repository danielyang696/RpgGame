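; Base Blueprint for area-of-effect blasts that handles their visual and audio feedback when triggered.
; Trigger runs the parent logic, then spawns the BlastEffect Niagara system attached to the root and plays BlastSound at the actor's location.
; The actor destroys itself when the effect finishes, or after a short delay if no effect is set.
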(event `self.Trigger`
  (`parent.Trigger`)
  (`self.Spawn Blast Effect`)
  (`self.Play Blast Audio`))

(event `Spawn Blast Effect`
  (bind _blast_effect (`self.Blast Effect`)
    (:`then`
      (`NiagaraFunctionLibrary.SpawnSystemAttached` _blast_effect (`self.DefaultSceneRoot`) "None" (0.0 0.0 0.0) (struct) "KeepRelativeOffset")
      (add `NiagaraComponent.OnSystemFinished` (`self.Niagara`) (delegate `System Finished`)))
    (:`else`
      (`KismetSystemLibrary.Delay` 1.0)
      (`self.K2_DestroyActor`))))

(event `System Finished`
  (params (PSystem :type "NiagaraComponent Object Reference"))
  (`self.K2_DestroyActor`))

(event `Play Blast Audio`
  (bind _blast_sound (`self.Blast Sound`)
    (:`then`
      (`GameplayStatics.PlaySoundAtLocation` _blast_sound (`self.K2_GetActorLocation`) (struct) 1.0 1.0 0.0 null null null null))
    (:`else`)))

(fn `UserConstructionScript`
  (`parent.UserConstructionScript`))