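; BP_AOE_Base is a base area-of-effect actor that detects pawns within a radius when triggered.
; Trigger runs a one-shot sphere overlap at the actor's location, optionally ignoring the instigator and drawing a debug sphere.
; Each hit is broadcast individually through the OnAOEOverlapActors dispatcher, so the base applies no effect itself.
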(event `self.ReceiveBeginPlay`)

(event `Trigger`
  (`self.SpawnAOESphere`))

(event `SpawnAOESphere`
  (if (`self.DrawDebugSphere`)
    (`KismetSystemLibrary.DrawDebugSphere` (`self.K2_GetActorLocation`) (`self.Radius`) 12 (struct :`R` 1.0 :`G` 1.0 :`B` 1.0 :`A` 1.0) 2.0))
  (bind _outactors (`KismetSystemLibrary.SphereOverlapActors` (`self.K2_GetActorLocation`) (`self.Radius`) (`|MakeArray` "ObjectTypeQuery3" :!type "EObjectTypeQuery Enum") null (select `bool` (`self.IgnoreInstigator`) :`true` (`|MakeArray` (`self.GetInstigator`) :!type "Actor Object Reference"))))
  (for _array_element _outactors
    (`self.OnAOEOverlapActors` _array_element)))

(fn `UserConstructionScript`)