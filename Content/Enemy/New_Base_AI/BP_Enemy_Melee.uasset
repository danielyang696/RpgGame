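; Sword-wielding melee enemy character with a three-step montage combo, weapon equip/unequip and selectable movement speeds.
; SwordAttack starts or queues attacks, and SwordAttackCombo advances the saved combo or resets it.
; A looping timer sphere-traces along the blade, sending throttled damage to "Damageable" actors, with blood and sound on success.
; Event dispatchers signal attack end and equip changes, while montage notifies toggle weapon visibility.
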(event `Start Sword Trace`
  ; Sword Trace
  (bind _returnvalue (`KismetSystemLibrary.K2_SetTimerDelegate` (delegate `Sword Trace Loop`) 0.01 true))
  (set `self.SwordTraceLoop` _returnvalue))

(event `Attack 1`
  ; Combo system
  ;; Attack1
  (`/Engine/EditorBlueprintResources/StandardMacros.DoOnce` false :!label _label
    (:`Completed`
      (`KismetSystemLibrary.Delay` 0.1)
      (`|PlayMontage` (`self.Mesh`) "/Game/Enemy/Animation/Attack1_Montage.Attack1_Montage" (`self.attackAnimSpeed`)
        (:`then`
          (set `self.AttackIndex` 1)
          (goto _label :!via `Reset`))
        (:`OnCompleted`
          _)
        (:`OnInterrupted`
          _))
      (`self.OnAttackEnd`))))

(event `Sword Trace Loop`
  ; Sword Trace
  (if (not (`/Game/Damage_System/BPC_DamageSystem.IsDead` (`self.BPC_DamageSystem`)))
    (bind (_outhit _returnvalue) (`KismetSystemLibrary.SphereTraceSingle` :`Start` (`SceneComponent.K2_GetComponentLocation` (`self.Sword bottom`)) :`End` (`SceneComponent.K2_GetComponentLocation` (`self.Sword top`)) :`Radius` 35.0 :`TraceChannel` "TraceTypeQuery1" :`DrawDebugType` "ForDuration" :`DrawTime` 0.05))
    (if _returnvalue
      (bind (_bblockinghit _binitialoverlap _time _distance _location _impactpoint _normal _impactnormal _physmat _hitactor) (`GameplayStatics.BreakHitResult` _outhit))
      (if (`self.ActorHasTag` _hitactor "Damageable")
        (`/Engine/EditorBlueprintResources/StandardMacros.DoOnce` false :!label _label_2
          (:`Completed`
            (bind _wasdamaged (message `/Game/Damage_System/BPI_Damagable.TakeDamage` _hitactor (make `/Game/Damage_System/S_DamageInfo` 20.0 "NewEnumerator1" "NewEnumerator0" false false false self)))
            (if _wasdamaged
              (`self.Play Hit Audio`)
              (`GameplayStatics.SpawnEmitterAtLocation` "/Game/FX/Particles/Blood/P_Blood_Splat_Cone.P_Blood_Splat_Cone" _location (`KismetMathLibrary.MakeRotFromXY` _normal _normal) (0.4 0.4 0.4) true "AutoRelease"))
            (`KismetSystemLibrary.Delay` 0.5)
            (goto _label_2 :!via `Reset`)))))))

(event `/Game/Enemy/New_Base_AI/AI/BPI_EnemyAI.DefaultAttack`
  (`|PlayMontage` (`self.Mesh`) "/Game/Enemy/Animation/Attack1_Montage.Attack1_Montage" (`self.attackAnimSpeed`)
    (:`OnCompleted`
      _)
    (:`OnInterrupted`
      _))
  (`self.OnAttackEnd`))

(event `Attack2`
  ; Combo system
  ;; Attack2
  (`/Engine/EditorBlueprintResources/StandardMacros.DoOnce` false :!label _label_3
    (:`Completed`
      (`KismetSystemLibrary.Delay` 0.1)
      (`|PlayMontage` (`self.Mesh`) "/Game/Enemy/Animation/Attack2_Montage.Attack2_Montage"
        (:`then`
          (set `self.AttackIndex` 2)
          (goto _label_3 :!via `Reset`))
        (:`OnCompleted`
          _)
        (:`OnInterrupted`
          _))
      (`self.OnAttackEnd`))))

(event `Sword Attack`
  ; Combo system
  ;; Sword Attack
  (if (`self.isAttacking`)
    (set `self.saveAttack?` true)
    (else
      (set `self.isAttacking` true)
      (switch `int` (`self.AttackIndex`) :!label _label_4
        (:`0`
          (`self.Attack 1`))
        (:`1`
          (`self.Attack2`))
        (:`2`
          (`self.Attack3`))))))

(event `Stop Sword Trace`
  ; Sword Trace
  (`KismetSystemLibrary.K2_ClearAndInvalidateTimerHandle` (`self.SwordTraceLoop`)))

(event `Sword Attack Combo`
  ; Combo system
  ;; Combo Continue
  (if (`self.saveAttack?`)
    (set `self.saveAttack?` false)
    (goto _label_4)
    (else
      (`self.Stop Combo`))))

(event `/Game/Enemy/New_Base_AI/AI/BPI_EnemyAI.EquipWeapon`
  ; Wield/Sheath Sword
  (bind _notifyname (`|PlayMontage` (`self.Mesh`) "/Game/Characters/RpgGame/Animation/Fight_Ready/AS_OneHand_Up_Fight_Ready_R_1_Montage.AS_OneHand_Up_Fight_Ready_R_1_Montage")
    (:`OnCompleted`
      (`self.EquipWeaponAssighByTask`)
      (set `self.isWieldSword` true))
    (:`OnNotifyBegin`
      (switch `name` _notifyname
        (:`Default`
          (`SceneComponent.SetVisibility` (`self.Weapon`) true false))))))

(event `Play Hit Audio`
  ; Hit Audio
  (`GameplayStatics.PlaySoundAtLocation` "/Game/Audio/Hit/Minecraft_dungeons_Sword_hit__1.Minecraft_dungeons_Sword_hit__1" (`self.K2_GetActorLocation` (`self.GetOwner`)) (struct) 1.0 1.0 0.0 "/Game/Audio/SA_Character.SA_Character" null null null))

(event `Attack3`
  ; Combo system
  ;; Attack3
  (`/Engine/EditorBlueprintResources/StandardMacros.DoOnce` false :!label _label_5
    (:`Completed`
      (`KismetSystemLibrary.Delay` 0.1)
      (`|PlayMontage` (`self.Mesh`) "/Game/Enemy/Animation/Attack3_Montage.Attack3_Montage"
        (:`then`
          (set `self.AttackIndex` 3)
          (goto _label_5 :!via `Reset`))
        (:`OnCompleted`
          _)
        (:`OnInterrupted`
          _))
      (`self.OnAttackEnd`))))

(event `/Game/Enemy/New_Base_AI/AI/BPI_EnemyAI.UnEquipWeapon`
  ; Wield/Sheath Sword
  (bind _notifyname (`|PlayMontage` (`self.Mesh`) "/Game/Characters/RpgGame/Animation/Fight_Ready/AS_OneHand_Up_Fight_End_R_1_Montage.AS_OneHand_Up_Fight_End_R_1_Montage")
    (:`OnCompleted`
      (`self.UnequipWeaponAssignByTask`)
      (set `self.isWieldSword` false))
    (:`OnNotifyBegin`
      (switch `name` _notifyname
        (:`Default`
          (`SceneComponent.SetVisibility` (`self.Weapon`) false false))))))

(event `Stop Combo`
  ; Combo system
  ;; Stop Combo/Attack
  (set `self.isAttacking` false)
  (set `self.AttackIndex` 0))

(fn `Set Movement Speed`
  (params (Speed :type "/Game/Enemy/New_Base_AI/AI/Enums/E_AI_MovementSpeed Enum" :default "NewEnumerator0"))
  (returns (SpeedValue :type "Float (double-precision)"))
  (bind _output_get (set `CharacterMovementComponent.MaxWalkSpeed` (select `/Game/Enemy/New_Base_AI/AI/Enums/E_AI_MovementSpeed` Speed :`NewEnumerator1` 120.0 :`NewEnumerator2` 475.0 :`NewEnumerator3` 650.0 :!type "Float (single-precision)") (`self.CharacterMovement`)))
  (return _output_get))

(fn `UserConstructionScript`
  (bind _bpc_damagesystem (`self.BPC_DamageSystem`))
  (`parent.UserConstructionScript`)
  (set `/Game/Damage_System/BPC_DamageSystem.MaxHealth` 100.0 _bpc_damagesystem)
  (set `/Game/Damage_System/BPC_DamageSystem.Health` 100.0 _bpc_damagesystem))