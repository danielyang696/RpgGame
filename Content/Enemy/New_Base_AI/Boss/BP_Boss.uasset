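; Boss enemy Blueprint built on a base AI enemy, with a large health pool, two melee sword combos and its own health bar widget.
; Attacks run through the attack system component, and taking damage refreshes the bar.
; Each parry freezes the AI and plays a stagger montage; reaching the parry limit triggers a knockdown that enables the front fatal collision.
; When either montage ends, the boss controller resumes attacking its last target.
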(event `self.ReceiveBeginPlay`
  (bind _bpc_damagesystem (`self.BPC_DamageSystem`))
  (`parent.ReceiveBeginPlay`)
  ; health bar
  (`WidgetComponent.SetWidget` (`self.Health Bar Widget`) null)
  (bind _returnvalue (`|CreateWidget` "/Game/UI/WB_BossHealthbar.WB_BossHealthbar_C"))
  (bind _output_get (set `self.HealthBar` _returnvalue))
  (`/Game/UI/WB_BossHealthbar.SetHealthBarPercetnage` _output_get (`/Game/Damage_System/BPC_DamageSystem.Health` _bpc_damagesystem) (`/Game/Damage_System/BPC_DamageSystem.MaxHealth` _bpc_damagesystem)))

(event `Attack Combo1`
  (params (AttackTarget :type "Actor Object Reference"))
  ; Attack
  (`/Game/Buleprints/BPC_AttackSystem.Short Range Attack` (`self.BPC_AttackSystem`) (make `/Game/Buleprints/EnumAndStructure/S_AttackInfo` AttackTarget "/Game/Enemy/New_Base_AI/Boss/Anim/Axe/Montages/Standing_Melee_Combo_Attack_Ver__1_Anim_Montage.Standing_Melee_Combo_Attack_Ver__1_Anim_Montage" (make `/Game/Damage_System/S_DamageInfo` 30.0 "NewEnumerator1" "NewEnumerator1" true true false self)) 50.0 (`self.Sword bottom`) (`self.Sword top`)))

(event `Attack Combo2`
  (params (AttackTarget :type "Actor Object Reference"))
  ; Attack
  (`/Game/Buleprints/BPC_AttackSystem.Short Range Attack` (`self.BPC_AttackSystem`) (make `/Game/Buleprints/EnumAndStructure/S_AttackInfo` AttackTarget "/Game/Enemy/New_Base_AI/Boss/Anim/Axe/Montages/Standing_Melee_Combo_Attack_Ver__2_Anim_Montage.Standing_Melee_Combo_Attack_Ver__2_Anim_Montage" (make `/Game/Damage_System/S_DamageInfo` 30.0 "NewEnumerator1" "NewEnumerator1" true true false self)) 50.0 (`self.Sword bottom`) (`self.Sword top`)))

(event `self.BPC_AttackSystem.OnBeParried`
  (bind _returnvalue (`self.GetController`))
  (bind _returnvalue_2 (`self.GetController`))
  ; be parried
  (`/Engine/EditorBlueprintResources/StandardMacros.IncrementInt` (`self.ParryCount`)
    (:`  `
      (if (>= (`self.ParryCount`) (`self.MaxParryCount`))
        (set `self.ParryCount` 0)
        (`GameplayStatics.PlaySoundAtLocation` "/Game/Audio/Shield/BlockBreak.BlockBreak" (`self.K2_GetActorLocation`) (struct) 2.0 0.6 0.0 null null null null)
        (`MovementComponent.StopMovementImmediately` (`self.CharacterMovement`))
        (`/Game/Enemy/New_Base_AI/AI/AIC_Enemy_Base.Set State as Frozen` (`self.AIC Enemy Base`))
        (`GameplayStatics.SpawnEmitterAtLocation` "/Game/FX_2/Particles/Sparks/P_Sparks_E.P_Sparks_E" (`SceneComponent.K2_GetComponentLocation` (`self.Sword bottom`)) (struct :`Roll` 90.0) (1.0 1.0 1.0) true "AutoRelease")
        (`|PlayMontage` (`self.Mesh`) "/Game/Characters/RpgGame/Animation/Shield/Montage/BeParried_Down_Montage.BeParried_Down_Montage"
          (:`then`
            (`PrimitiveComponent.SetCollisionEnabled` (`self.FrontFatalCollision`) "QueryOnly"))
          (:`OnCompleted`
            (`PrimitiveComponent.SetCollisionEnabled` (`self.FrontFatalCollision`) "NoCollision" :!label _label)
            (`/Engine/EditorBlueprintResources/StandardMacros.IsValid` _returnvalue
              (:`Is Valid`
                _)
              (:`Is Not Valid`
                (`KismetSystemLibrary.DelayUntilNextTick`)))
            (`/Game/Enemy/New_Base_AI/AI/AIC_Enemy_Base.Set State as Attacking` (cast `/Game/Enemy/New_Base_AI/Boss/AIC_Enemy_Boss` _returnvalue :!pure true) null true))
          (:`OnInterrupted`
            (goto _label)))
        (else
          (`GameplayStatics.PlaySoundAtLocation` "/Game/Audio/Shield/BlockBreak.BlockBreak" (`self.K2_GetActorLocation`) (struct) 0.8 1.3 0.0 null null null null)
          (`MovementComponent.StopMovementImmediately` (`self.CharacterMovement`))
          (`/Game/Enemy/New_Base_AI/AI/AIC_Enemy_Base.Set State as Frozen` (`self.AIC Enemy Base`))
          (`GameplayStatics.SpawnEmitterAtLocation` "/Game/FX_2/Particles/Sparks/P_Sparks_E.P_Sparks_E" (`SceneComponent.K2_GetComponentLocation` (`self.Sword bottom`)) (struct) (0.7 0.7 0.7) true "AutoRelease")
          (`|PlayMontage` (`self.Mesh`) "/Game/Characters/RpgGame/Animation/Shield/Montage/BeParried_Montage.BeParried_Montage"
            (:`OnCompleted`
              _)
            (:`OnInterrupted`
              _))
          (`/Engine/EditorBlueprintResources/StandardMacros.IsValid` _returnvalue_2
            (:`Is Valid`
              (set `/Game/Damage_System/BPC_DamageSystem.IsInterruptible` true (`self.BPC_DamageSystem`))
              (`KismetSystemLibrary.Delay` 0.5)
              (`/Game/Enemy/New_Base_AI/AI/AIC_Enemy_Base.Set State as Attacking` (cast `/Game/Enemy/New_Base_AI/Boss/AIC_Enemy_Boss` _returnvalue_2 :!pure true) null true))))))))

(fn `Get Ideal Range`
  (returns (AttackRadius :type "Float (double-precision)") (DefendRadius :type "Float (double-precision)"))
  (return 200.0 400.0))

(fn `Set Movement Speed`
  (params (Speed :type "/Game/Enemy/New_Base_AI/AI/Enums/E_AI_MovementSpeed Enum" :default "NewEnumerator0"))
  (returns (SpeedValue :type "Float (double-precision)"))
  (set `CharacterMovementComponent.MaxWalkSpeed` (select `/Game/Enemy/New_Base_AI/AI/Enums/E_AI_MovementSpeed` Speed :`NewEnumerator1` 125.0 :`NewEnumerator2` 475.0 :`NewEnumerator3` 650.0 :!type "Float (single-precision)") (`self.CharacterMovement`))
  (return 0.0))

(fn `TakeDamage`
  (params (DamageInfo :type "/Game/Damage_System/S_DamageInfo Structure"))
  (returns (WasDamaged :type Boolean) (ParrySucces :type Boolean))
  (bind _bpc_damagesystem (`self.BPC_DamageSystem`))
  (bind _wasdamaged (`parent.TakeDamage` DamageInfo))
  (`/Game/UI/WB_BossHealthbar.SetHealthBarPercetnage` (`self.HealthBar`) (`/Game/Damage_System/BPC_DamageSystem.Health` _bpc_damagesystem) (`/Game/Damage_System/BPC_DamageSystem.MaxHealth` _bpc_damagesystem))
  (return _wasdamaged false))

(fn `UserConstructionScript`
  (bind _bpc_damagesystem (`self.BPC_DamageSystem`))
  (`parent.UserConstructionScript`)
  (bind _output_get (set `/Game/Damage_System/BPC_DamageSystem.MaxHealth` 1000.0 _bpc_damagesystem))
  (set `/Game/Damage_System/BPC_DamageSystem.Health` _output_get _bpc_damagesystem))