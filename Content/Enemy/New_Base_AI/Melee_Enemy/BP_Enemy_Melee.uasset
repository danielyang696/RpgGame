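; Sword-wielding melee enemy Blueprint built on the enemy AI base, providing attacks, blocking, parry reactions and weapon equip.
; Attack events pass montage and damage info to the attack system component, which handles sword traces and ground smash.
; Blockable hits outside attacks roll a block chance; blocking returns an attack token to the player and runs on a timer.
; Being parried freezes the AI and enables a front fatal collision until the montage ends.
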(event `self.ReceiveBeginPlay`
  (`parent.ReceiveBeginPlay`))

(event `GroundSmashAttack`
  (params (AttackTarget :type "Actor Object Reference"))
  ; Sword attack
  (`/Game/Buleprints/BPC_AttackSystem.GroundSmash` (`self.BPC_AttackSystem`) (make `/Game/Buleprints/EnumAndStructure/S_AttackInfo` AttackTarget "/Game/Enemy/Animation/Mixamo/Montages/GroundSmash_Montage.GroundSmash_Montage" (make `/Game/Damage_System/S_DamageInfo` 30.0 "NewEnumerator3" "NewEnumerator1" false false false self)) 200.0))

(event `Short Range Attack`
  (params (AttackTarget :type "Actor Object Reference"))
  ; Sword attack
  (`/Game/Buleprints/BPC_AttackSystem.Short Range Attack` (`self.BPC_AttackSystem`) (make `/Game/Buleprints/EnumAndStructure/S_AttackInfo` AttackTarget "/Game/Enemy/Animation/Attack1_Montage.Attack1_Montage" (make `/Game/Damage_System/S_DamageInfo` 15.0 "NewEnumerator1" "NewEnumerator1" true true false self)) 30.0 (`self.Sword bottom`) (`self.Sword top`)))

(event `Long Range Jump Attack`
  (params (AttackTarget :type "Actor Object Reference"))
  ; Sword attack
  (`/Game/Buleprints/BPC_AttackSystem.Long Range Jump Attack` (`self.BPC_AttackSystem`) (make `/Game/Buleprints/EnumAndStructure/S_AttackInfo` AttackTarget "/Game/Enemy/Animation/Mixamo/Montages/MM_Standing_Melee_Run_Jump_Attack_Anim_Montage.MM_Standing_Melee_Run_Jump_Attack_Anim_Montage" (make `/Game/Damage_System/S_DamageInfo` 30.0 "NewEnumerator1" "NewEnumerator1" true true false self)) 60.0 (`self.Sword bottom`) (`self.Sword top`)))

(event `Start Sword Trace`
  (params (DamageInfo :type "/Game/Damage_System/S_DamageInfo Structure"))
  ; Sword Trace
  (`/Game/Buleprints/BPC_AttackSystem.Sword Trace Start` (`self.BPC_AttackSystem`) (`self.Sword bottom`) (`self.Sword top`) DamageInfo 30.0))

(event `Stop Sword Trace`
  ; Sword Trace
  (`/Game/Buleprints/BPC_AttackSystem.Sword Trace End` (`self.BPC_AttackSystem`)))

(event `/Game/Enemy/New_Base_AI/AI/BPI_EnemyAI.EquipWeapon`
  ; Wield/Sheath Sword
  (bind _notifyname (`|PlayMontage` (`self.Mesh`) "/Game/Characters/RpgGame/Animation/Fight_Ready/AS_OneHand_Up_Fight_Ready_R_1_Montage.AS_OneHand_Up_Fight_Ready_R_1_Montage" 1.0 0.0 "None" false)
    (:`OnCompleted`
      (`self.EquipWeaponAssighByTask` :!label _label)
      (set `self.isWieldSword` true))
    (:`OnInterrupted`
      (goto _label))
    (:`OnNotifyBegin`
      (switch `name` _notifyname
        (:`Default`
          (`SceneComponent.SetVisibility` (`self.Weapon`) true false))))))

(event `/Game/Enemy/New_Base_AI/AI/BPI_EnemyAI.UnEquipWeapon`
  ; Wield/Sheath Sword
  (bind _notifyname (`|PlayMontage` (`self.Mesh`) "/Game/Characters/RpgGame/Animation/Fight_Ready/AS_OneHand_Up_Fight_End_R_1_Montage.AS_OneHand_Up_Fight_End_R_1_Montage" 1.0 0.0 "None" false)
    (:`OnCompleted`
      (`self.UnequipWeaponAssignByTask`)
      (set `self.isWieldSword` false))
    (:`OnNotifyBegin`
      (switch `name` _notifyname
        (:`Default`
          (`SceneComponent.SetVisibility` (`self.Weapon`) false false))))))

(event `StartBlock`
  ; Block
  (message `/Game/Damage_System/BPI_Damagable.ReturnAttackToken` (`GameplayStatics.GetPlayerPawn` 0) 1)
  (`KismetSystemLibrary.K2_ClearAndInvalidateTimerHandle` (`self.HoldBlockTimer`))
  (set `self.BlockState` "NewEnumerator1")
  (set `/Game/Damage_System/BPC_DamageSystem.IsBlocking` true (`self.BPC_DamageSystem`))
  (bind _returnvalue (`KismetSystemLibrary.K2_SetTimerDelegate` (`|CreateDelegate` :!event `EndBlock`) 2.0))
  (set `self.HoldBlockTimer` _returnvalue))

(event `self.BPC_DamageSystem.OnBlocked`
  (params (NewParam :type "/Game/Damage_System/S_DamageInfo Structure"))
  ; Block
  (set `self.BlockState` "NewEnumerator2")
  (`KismetSystemLibrary.K2_ClearAndInvalidateTimerHandle` (`self.HoldBlockTimer`))
  (bind _notifyname (`|PlayMontage` (`self.Mesh`) "/Game/Enemy/Animation/Mixamo/Montages/MM_Standing_Block_React_Large_Anim_Montage.MM_Standing_Block_React_Large_Anim_Montage")
    (:`then`
      (`self.LaunchCharacter` (* (`self.GetActorForwardVector`) -1000.0) true))
    (:`OnCompleted`
      (`self.EndBlock` :!label _label_2))
    (:`OnInterrupted`
      (goto _label_2))
    (:`OnNotifyBegin`
      (switch `name` _notifyname
        (:`Default`
          (`GameplayStatics.PlaySoundAtLocation` "/Game/Audio/soundnotfrown-sword-hit-416334.soundnotfrown-sword-hit-416334" (`self.K2_GetActorLocation`) (struct) 0.5 (`KismetMathLibrary.RandomFloatInRange` 0.8 1.1) 0.0 "/Game/Audio/SA_Character.SA_Character" null null null))))))

(event `EndBlock`
  ; Block
  (set `/Game/Damage_System/BPC_DamageSystem.IsBlocking` false (`self.BPC_DamageSystem`))
  (set `self.BlockState` "NewEnumerator0")
  (`self.OnBlockEnd`))

(event `self.BPC_AttackSystem.OnBeParried`
  (bind _returnvalue (`self.GetController`))
  (`MovementComponent.StopMovementImmediately` (`self.CharacterMovement`))
  (`/Game/Enemy/New_Base_AI/AI/AIC_Enemy_Base.Set State as Frozen` (`self.AIC Enemy Base`))
  (`GameplayStatics.SpawnEmitterAtLocation` "/Game/FX_2/Particles/Sparks/P_Sparks_E.P_Sparks_E" (`SceneComponent.K2_GetComponentLocation` (`self.Sword bottom`)) (struct :`Roll` 90.0) (1.0 1.0 1.0) true "AutoRelease")
  (`|PlayMontage` (`self.Mesh`) "/Game/Characters/RpgGame/Animation/Shield/Montage/BeParried_Down_Montage.BeParried_Down_Montage"
    (:`then`
      (`PrimitiveComponent.SetCollisionEnabled` (`self.FrontFatalCollision`) "QueryOnly"))
    (:`OnCompleted`
      (`PrimitiveComponent.SetCollisionEnabled` (`self.FrontFatalCollision`) "NoCollision" :!label _label_3)
      (`/Engine/EditorBlueprintResources/StandardMacros.IsValid` _returnvalue
        (:`Is Valid`
          _)
        (:`Is Not Valid`
          (`KismetSystemLibrary.DelayUntilNextTick`)))
      (`/Game/Enemy/New_Base_AI/AI/AIC_Enemy_Base.Set State as Attacking` (cast `/Game/Enemy/New_Base_AI/AI/AIC_Enemy_Base` _returnvalue :!pure true) null true))
    (:`OnInterrupted`
      (goto _label_3))))

(fn `Get Ideal Range`
  (returns (AttackRadius :type "Float (double-precision)") (DefendRadius :type "Float (double-precision)"))
  (return 200.0 600.0))

(fn `IsDead`
  (returns (Dead :type Boolean))
  (return false))

(fn `Set Movement Speed`
  (params (Speed :type "/Game/Enemy/New_Base_AI/AI/Enums/E_AI_MovementSpeed Enum" :default "NewEnumerator0"))
  (returns (SpeedValue :type "Float (double-precision)"))
  (bind _output_get (set `CharacterMovementComponent.MaxWalkSpeed` (select `/Game/Enemy/New_Base_AI/AI/Enums/E_AI_MovementSpeed` Speed :`NewEnumerator1` 125.0 :`NewEnumerator2` 475.0 :`NewEnumerator3` 650.0 :!type "Float (single-precision)") (`self.CharacterMovement`)))
  (return _output_get))

(fn `TakeDamage`
  (params (DamageInfo :type "/Game/Damage_System/S_DamageInfo Structure"))
  (returns (WasDamaged :type Boolean) (ParrySucces :type Boolean))
  (if (and (`.CanBeBlocked_12_002F20124017856AB5D7E5B2E16A4929` (break `/Game/Damage_System/S_DamageInfo` DamageInfo)) (not (`self.isAttacking`)))
    (`self.TryToBlock`))
  (bind _wasdamaged (`/Game/Damage_System/BPC_DamageSystem.TakeDamage` (`self.BPC_DamageSystem`) DamageInfo))
  (return _wasdamaged false))

(fn `TryToBlock`
  (if (<= (`KismetMathLibrary.RandomFloat`) (`self.BlockChance`))
    (`self.StartBlock`)))

(fn `UserConstructionScript`
  (bind _bpc_damagesystem (`self.BPC_DamageSystem`))
  (`parent.UserConstructionScript`)
  (set `/Game/Damage_System/BPC_DamageSystem.MaxHealth` 100.0 _bpc_damagesystem)
  (set `/Game/Damage_System/BPC_DamageSystem.Health` 100.0 _bpc_damagesystem))