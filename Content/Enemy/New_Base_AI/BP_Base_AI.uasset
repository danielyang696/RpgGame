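; Base enemy AI character that forwards health, damage and attack-token interface calls to its damage component and shows a health bar widget.
; Hit responses freeze the AI, play a random montage with knockback, then set it attacking the damage causer.
; Attacks reserve tokens from targets and return them on attack end or death.
; Death stops AI logic and ragdolls the mesh; other functions supply patrol route, team, ranges, movement speeds and back-fatal animation.
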(event `self.ReceiveBeginPlay`
  (bind _bpc_damagesystem (`self.BPC_DamageSystem`))
  (bind _asaic_enemy_base (cast `/Game/Enemy/New_Base_AI/AI/AIC_Enemy_Base` (`AIBlueprintHelperLibrary.GetAIController` self)))
  (set `self.AIC Enemy Base` _asaic_enemy_base)
  (bind _returnvalue (`|CreateWidget` "/Game/UI/WB_DummyHealthBar.WB_DummyHealthBar_C" null self))
  (`WidgetComponent.SetWidget` (`self.Health Bar Widget`) _returnvalue)
  (add `/Game/Damage_System/BPC_DamageSystem.OnDeath` _bpc_damagesystem (`|CreateDelegate` :!event `On Death`))
  (add `/Game/Damage_System/BPC_DamageSystem.OnDamageResponse` _bpc_damagesystem (`|CreateDelegate` :!event `OnDamageResponse_Event`)))

(event `On Death`
  (bind _aic_enemy_base (`self.AIC Enemy Base`))
  (bind _reservedattacktokens (`self.ReservedAttackTokens`))
  (`BrainComponent.StopLogic` (`AIController.BrainComponent` _aic_enemy_base) "")
  (`/Game/Enemy/New_Base_AI/AI/AIC_Enemy_Base.Set State as Dead` _aic_enemy_base)
  (if (`BlueprintMapLibrary.Map_IsEmpty` (`self.ReservedAttackTokens`))
    (`PrimitiveComponent.SetSimulatePhysics` (`self.Mesh`) true :!label _label)
    (`KismetSystemLibrary.Delay` 0.2)
    (`GameplayStatics.PlaySoundAtLocation` "/Game/Audio/Grunt/SC_Death.SC_Death" (`self.K2_GetActorLocation`) (struct) 1.0 1.0 0.0 null null null null)
    (`SceneComponent.SetVisibility` (`self.Health Bar Widget`) false false)
    (`CharacterMovementComponent.SetMovementMode` (`self.CharacterMovement`) "MOVE_None" 0)
    (`PrimitiveComponent.SetCollisionEnabled` (`self.CapsuleComponent`) "NoCollision")
    (`KismetArrayLibrary.Array_Remove` (`self.Tags`))
    (else
      ; Return all attack tokens
      (bind _keys (`BlueprintMapLibrary.Map_Keys` _reservedattacktokens))
      (for _array_element _keys
        (message `/Game/Damage_System/BPI_Damagable.ReturnAttackToken` _array_element (`BlueprintMapLibrary.Map_Find` _reservedattacktokens _array_element))
        (goto _label)))))

(event `OnDamageResponse_Event`
  (params (DamageRespones :type "/Game/Damage_System/E_DamageResponse Enum" :default "NewEnumerator0") (DamageCauser :type "Actor Object Reference"))
  (bind _returnvalue_location (`KismetMathLibrary.BreakTransform` (`self.GetTransform` DamageCauser)))
  (bind _returnvalue_location_2 (`KismetMathLibrary.BreakTransform` (`self.GetTransform`)))
  (switch `/Game/Damage_System/E_DamageResponse` DamageRespones
    (:`NewEnumerator0`
      _)
    (:`NewEnumerator1`
      _))
  (`MovementComponent.StopMovementImmediately` (`self.CharacterMovement`))
  (`/Game/Enemy/New_Base_AI/AI/AIC_Enemy_Base.Set State as Frozen` (`self.AIC Enemy Base`))
  (`|PlayMontage` (`self.Mesh`) (`KismetArrayLibrary.Array_Random` (`self.Hit_AnimMontage`))
    (:`then`
      (`self.LaunchCharacter` (* (`KismetMathLibrary.Normal` (`KismetMathLibrary.MakeVector` (.x (- _returnvalue_location_2 _returnvalue_location)) (.y (- _returnvalue_location_2 _returnvalue_location))) 1.0) 1000.0) true))
    (:`OnCompleted`
      (`/Game/Enemy/New_Base_AI/AI/AIC_Enemy_Base.Set State as Attacking` (`self.AIC Enemy Base`) DamageCauser true :!label _label_2))
    (:`OnInterrupted`
      (goto _label_2))))

(event `Ragdoll`
  ; Ragdoll (enable simulate physics when target die
  (`|ExecutionSequence`
    (:`then_0`
      (`KismetSystemLibrary.Delay` 2.8)
      (`PrimitiveComponent.SetSimulatePhysics` (`self.Mesh`) true))
    (:`then_1`
      (`KismetSystemLibrary.Delay` 1.0)
      (`GameplayStatics.PlaySoundAtLocation` "/Game/Audio/Grunt/SC_Death.SC_Death" (`self.K2_GetActorLocation`) (struct) 1.0 1.0 0.0 null null null null))))

(event `/Game/Enemy/New_Base_AI/AI/BPI_EnemyAI.DefaultAttack`
  (params (AttackTarget :type "Actor Object Reference"))
  (set `self.isAttacking` true))

(event `/Game/Damage_System/BPI_Damagable.ReturnAttackToken`
  (params (Amount :type Integer))
  (`/Game/Damage_System/BPC_DamageSystem.ReturnAttackToken` (`self.BPC_DamageSystem`) Amount))

(event `/Game/Enemy/New_Base_AI/AI/BPI_EnemyAI.StoredAttackTokens`
  (params (AttackTarget :type "Actor Object Reference") (Amount :type Integer))
  (bind (_value _returnvalue) (`BlueprintMapLibrary.Map_Find` (`self.ReservedAttackTokens`) AttackTarget))
  (`BlueprintMapLibrary.Map_Add` (`self.ReservedAttackTokens`) AttackTarget (`KismetMathLibrary.SelectInt` (+ Amount _value) Amount _returnvalue)))

(event `/Game/Enemy/New_Base_AI/AI/BPI_EnemyAI.AttackEnd`
  (params (AttackTarget :type "Actor Object Reference"))
  (bind _tokensuseincurrentattack (`self.TokensUseInCurrentAttack`))
  (message `/Game/Damage_System/BPI_Damagable.ReturnAttackToken` AttackTarget _tokensuseincurrentattack)
  (`/Game/Enemy/New_Base_AI/AI/BPI_EnemyAI.StoredAttackTokens` AttackTarget (* _tokensuseincurrentattack -1))
  (set `self.isAttacking` false)
  (`self.OnAttackEnd`))

(fn `Attack`
  (returns (animationDuration :type "Float (double-precision)")))

(fn `BackFatal`
  (returns (refLocation :type "Vector Structure") (fatalRotation :type "Rotator Structure"))
  (`self.PlayAnimMontage` "/Game/Characters/RpgGame/Animation/Fatal/AS_OneHand_Up_Fatal_Hit_1_Montage.AS_OneHand_Up_Fatal_Hit_1_Montage")
  (return (`SceneComponent.K2_GetComponentLocation` (`self.ref location`)) (`KismetMathLibrary.MakeRotator` (.roll (`self.K2_GetActorRotation`)) (.pitch (`self.K2_GetActorRotation`)) (+ (.yaw (`self.K2_GetActorRotation`)) 30.0))))

(fn `Get Ideal Range`
  (returns (AttackRadius :type "Float (double-precision)") (DefendRadius :type "Float (double-precision)"))
  (return 150.0 350.0))

(fn `Get Patrol Route`
  (returns (PatrolRoute :type "/Game/Enemy/New_Base_AI/AI/BP_PatrolRoute Object Reference"))
  (return (`self.BP_PatrolRoute`)))

(fn `GetCurrentHealth`
  (returns (Health :type "Float (double-precision)"))
  (return (`/Game/Damage_System/BPC_DamageSystem.Health` (`self.BPC_DamageSystem`))))

(fn `GetIsAttacking`
  (returns (IsAttacking :type Boolean))
  (return (`self.isAttacking`)))

(fn `GetMaxHealth`
  (returns (MaxHealth :type "Float (double-precision)"))
  (return (`/Game/Damage_System/BPC_DamageSystem.MaxHealth` (`self.BPC_DamageSystem`))))

(fn `GetTeamNumber`
  (returns (TeamNumber :type Integer))
  (return (`self.TeamNumber`)))

(fn `Heal`
  (params (Amount :type "Float (double-precision)"))
  (returns (NewHealth :type "Float (double-precision)"))
  (bind _newhealth (`/Game/Damage_System/BPC_DamageSystem.Heal` (`self.BPC_DamageSystem`) Amount))
  (return _newhealth))

(fn `IsDead`
  (returns (Dead :type Boolean))
  (return (`/Game/Damage_System/BPC_DamageSystem.IsDead` (`self.BPC_DamageSystem`))))

(fn `ReserveAttackToken`
  (params (Amount :type Integer))
  (returns (success :type Boolean))
  (bind _success (`/Game/Damage_System/BPC_DamageSystem.ReserveAttackToken` (`self.BPC_DamageSystem`) Amount))
  (return _success))

(fn `Set Movement Speed`
  (params (Speed :type "/Game/Enemy/New_Base_AI/AI/Enums/E_AI_MovementSpeed Enum" :default "NewEnumerator0"))
  (returns (SpeedValue :type "Float (double-precision)"))
  (bind _output_get (set `CharacterMovementComponent.MaxWalkSpeed` (select `/Game/Enemy/New_Base_AI/AI/Enums/E_AI_MovementSpeed` Speed :`NewEnumerator1` 125.0 :`NewEnumerator2` 475.0 :`NewEnumerator3` 650.0 :!type "Float (single-precision)") (`self.CharacterMovement`)))
  (return _output_get))

(fn `StartAttack`
  (params (AttackTarget :type "Actor Object Reference") (Amount :type Integer))
  (returns (Success :type Boolean))
  (bind _success (message `/Game/Damage_System/BPI_Damagable.ReserveAttackToken` AttackTarget Amount))
  (if _success
    (`/Game/Enemy/New_Base_AI/AI/BPI_EnemyAI.StoredAttackTokens` AttackTarget Amount)
    (set `self.TokensUseInCurrentAttack` Amount)
    (return true)
    (else
      (return false))))

(fn `TakeDamage`
  (params (DamageInfo :type "/Game/Damage_System/S_DamageInfo Structure"))
  (returns (WasDamaged :type Boolean))
  (bind _wasdamaged (`/Game/Damage_System/BPC_DamageSystem.TakeDamage` (`self.BPC_DamageSystem`) DamageInfo))
  (return _wasdamaged))

(fn `UserConstructionScript`)