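; BP_AI_Boss is a boss enemy pawn that extends a parent AI class and links its health and death to BP_AIController_Boss.
; On BeginPlay it caches the boss controller and passes it max health from the player stat component.
; Tick copies current health to the controller every frame.
; After parent damage handling, AnyDamage tells the controller to deactivate the boss fight if IsDead is set.
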(event `self.ReceiveBeginPlay`
  (`parent.ReceiveBeginPlay`)
  (bind _asbp_aicontroller_boss (cast `/Game/Enemy/Boss/BP_AIController_Boss` (`self.GetController`)))
  (bind _output_get (set `self.BP AIController Boss` _asbp_aicontroller_boss))
  (set `/Game/Enemy/Boss/BP_AIController_Boss.maxHealth` (`/Game/Buleprints/BPC_PlayerStat.maxHealth` (`self.BPC_PlayerStat`)) _output_get))

(event `self.ReceiveTick`
  (params (DeltaSeconds :type "Float (single-precision)"))
  (`parent.ReceiveTick` DeltaSeconds)
  (set `/Game/Enemy/Boss/BP_AIController_Boss.currentHealth` (`/Game/Buleprints/BPC_PlayerStat.currentHealth` (`self.BPC_PlayerStat`)) (`self.BP AIController Boss`)))

(event `self.ReceiveAnyDamage`
  (params (Damage :type "Float (single-precision)") (DamageType :type "DamageType Object Reference") (InstigatedBy :type "Controller Object Reference") (DamageCauser :type "Actor Object Reference"))
  (`parent.ReceiveAnyDamage` Damage DamageType InstigatedBy DamageCauser)
  (if (`self.IsDead`)
    (`/Game/Enemy/Boss/BP_AIController_Boss.Deactivate Boss Fight` (`self.BP AIController Boss`))))

(fn `UserConstructionScript`
  (`parent.UserConstructionScript`))