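; BP_AI is a sword-fighting enemy with a camera-facing health bar, a behavior-tree-driven three-hit combo and ragdoll death.
; Attack montages chain through a saved-attack flag, while a looping-timer sphere trace along the blade damages "Damageable" actors.
; Incoming damage cancels the combo, plays a random reaction, knocks it away from the player and updates BPCPlayerStat, which decides death.
; BackFatal plays a fatal-hit montage and returns a reference location and rotation.
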(event `self.ReceiveBeginPlay`
  (bind _aswb_dummy_health_bar (cast `/Game/UI/WB_DummyHealthBar` (`WidgetComponent.GetWidget` (`self.Health Bar Widget`))))
  (set `self.HealthBarUI` _aswb_dummy_health_bar))

(event `self.ReceiveTick`
  (params (DeltaSeconds :type "Float (single-precision)"))
  (`SceneComponent.K2_SetWorldRotation` (`self.Health Bar Widget`) (`KismetMathLibrary.FindLookAtRotation` (`SceneComponent.K2_GetComponentLocation` (`self.Health Bar Widget`)) (`SceneComponent.K2_GetComponentLocation` (`PlayerCameraManager.TransformComponent` (`GameplayStatics.GetPlayerCameraManager` 0)))) false false))

(event `Ragdoll`
  ; Ragdoll (enable simulate physics when target die
  (`|ExecutionSequence`
    (:`then_0`
      (`KismetSystemLibrary.Delay` 2.8)
      (`PrimitiveComponent.SetSimulatePhysics` (`self.Mesh`) true))
    (:`then_1`
      (`KismetSystemLibrary.Delay` 1.0)
      (`GameplayStatics.PlaySoundAtLocation` "/Game/Audio/Grunt/SC_Death.SC_Death" (`self.K2_GetActorLocation`) (struct) 1.0 1.0 0.0 null null null null))))

(event `self.ReceiveAnyDamage`
  (params (Damage :type "Float (single-precision)") (DamageType :type "DamageType Object Reference") (InstigatedBy :type "Controller Object Reference") (DamageCauser :type "Actor Object Reference"))
  (bind _returnvalue_location (`KismetMathLibrary.BreakTransform` (`self.GetTransform`)))
  ; take damage
  (if (not (`self.IsDead`))
    (`self.Stop Combo`)
    (`self.PlayAnimMontage` (`|GetArrayItem` (`self.Hit_AnimMontage`) (`KismetMathLibrary.RandomIntegerInRange` 0 (- (`KismetArrayLibrary.Array_Length` (`self.Hit_AnimMontage`)) 1))))
    (bind _asbp_third_person_character (cast `/Game/ThirdPerson/Blueprints/BP_ThirdPersonCharacter` (`GameplayStatics.GetPlayerCharacter` 0)))
    (bind _returnvalue_location_2 (`KismetMathLibrary.BreakTransform` (`self.GetTransform` _asbp_third_person_character)))
    (`CharacterMovementComponent.AddImpulse` (`self.CharacterMovement`) (* (`KismetMathLibrary.Normal` (`KismetMathLibrary.MakeVector` (.x (- _returnvalue_location _returnvalue_location_2)) (.y (- _returnvalue_location _returnvalue_location_2))) 1.0) 2200.0) true)
    (bind _isplayerdie (`/Game/Buleprints/BPC_PlayerStamina.DecreaseHealth` (`self.BPC_PlayerStat`) Damage))
    (bind _output_get (set `self.IsDead` _isplayerdie))
    (if _output_get
      (`PrimitiveComponent.SetSimulatePhysics` (`self.Mesh`) true)
      (`KismetSystemLibrary.Delay` 0.2)
      (`GameplayStatics.PlaySoundAtLocation` "/Game/Audio/Grunt/SC_Death.SC_Death" (`self.K2_GetActorLocation`) (struct) 1.0 1.0 0.0 null null null null)
      (`SceneComponent.SetVisibility` (`self.Health Bar Widget`) false false)
      (`CharacterMovementComponent.SetMovementMode` (`self.CharacterMovement`) "MOVE_None" 0)
      (`PrimitiveComponent.SetCollisionEnabled` (`self.CapsuleComponent`) "NoCollision")
      (`KismetArrayLibrary.Array_Remove` (`self.Tags`)))))

(event `Start Sword Trace`
  ; Sword Trace
  (bind _returnvalue (`KismetSystemLibrary.K2_SetTimerDelegate` (delegate `Sword Trace Loop`) 0.01 true))
  (set `self.SwordTraceLoop` _returnvalue))

(event `Attack 1`
  ; Combo system
  ;; Attack1
  (`/Engine/EditorBlueprintResources/StandardMacros.DoOnce` false :!label _label
    (:`Completed`
      (`KismetSystemLibrary.Delay` 0.1)
      (`|PlayMontage` (`self.Mesh`) "/Game/Enemy/Animation/Attack1_Montage.Attack1_Montage" (`self.attackAnimSpeed`)
        (:`then`
          (set `self.AttackIndex` 1)
          (goto _label :!via `Reset`))))))

(event `Sword Attack combo call from BT`
  ; Combo system
  ;; Attack Input
  (if (`self.canAttack`)
    (`self.Sword Attack`)))

(event `Sword Trace Loop`
  ; Sword Trace
  (if (not (`self.IsDead`))
    (bind (_outhit _returnvalue) (`KismetSystemLibrary.SphereTraceSingle` :`Start` (`SceneComponent.K2_GetComponentLocation` (`self.Sword bottom`)) :`End` (`SceneComponent.K2_GetComponentLocation` (`self.Sword top`)) :`Radius` 35.0 :`TraceChannel` "TraceTypeQuery1" :`DrawTime` 0.05))
    (if _returnvalue
      (bind (_bblockinghit _binitialoverlap _time _distance _location _impactpoint _normal _impactnormal _physmat _hitactor) (`GameplayStatics.BreakHitResult` _outhit))
      (if (`self.ActorHasTag` _hitactor "Damageable")
        (`/Engine/EditorBlueprintResources/StandardMacros.DoOnce` false :!label _label_2
          (:`Completed`
            (`GameplayStatics.ApplyDamage` _hitactor 20.0 null self)
            (`self.Play Hit Audio`)
            (`GameplayStatics.SpawnEmitterAtLocation` "/Game/FX/Particles/Blood/P_Blood_Splat_Cone.P_Blood_Splat_Cone" _location (`KismetMathLibrary.MakeRotFromXY` _normal _normal) (0.4 0.4 0.4) true "AutoRelease")
            (`KismetSystemLibrary.Delay` 0.5)
            (goto _label_2 :!via `Reset`)))))))

(event `Attack2`
  ; Combo system
  ;; Attack2
  (`/Engine/EditorBlueprintResources/StandardMacros.DoOnce` false :!label _label_3
    (:`Completed`
      (`KismetSystemLibrary.Delay` 0.1)
      (`|PlayMontage` (`self.Mesh`) "/Game/Enemy/Animation/Attack2_Montage.Attack2_Montage"
        (:`then`
          (set `self.AttackIndex` 2)
          (goto _label_3 :!via `Reset`))))))

(event `Sword Attack`
  ; Combo system
  ;; Sword Attack
  (if (`self.isAttacking`)
    (set `self.saveAttack?` true)
    (else
      (set `self.isAttacking` true)
      (switch `int` (`self.AttackIndex`) :!label _label_4
        (:`0`
          (`self.Attack 1`))
        (:`1`
          (`self.Attack2`))
        (:`2`
          (`self.Attack3`))))))

(event `Stop Sword Trace`
  ; Sword Trace
  (`KismetSystemLibrary.K2_ClearAndInvalidateTimerHandle` (`self.SwordTraceLoop`)))

(event `Play Hit Audio`
  ; Hit Audio
  (`GameplayStatics.PlaySoundAtLocation` "/Game/Audio/Hit/Minecraft_dungeons_Sword_hit__1.Minecraft_dungeons_Sword_hit__1" (`self.K2_GetActorLocation` (`self.GetOwner`)) (struct) 1.0 1.0 0.0 "/Game/Audio/SA_Character.SA_Character" null null null))

(event `Sword Attack Combo`
  ; Combo system
  ;; Combo Continue
  (if (`self.saveAttack?`)
    (set `self.saveAttack?` false)
    (goto _label_4)
    (else
      (`self.Stop Combo`))))

(event `Attack3`
  ; Combo system
  ;; Attack3
  (`/Engine/EditorBlueprintResources/StandardMacros.DoOnce` false :!label _label_5
    (:`Completed`
      (`KismetSystemLibrary.Delay` 0.1)
      (`|PlayMontage` (`self.Mesh`) "/Game/Enemy/Animation/Attack3_Montage.Attack3_Montage"
        (:`then`
          (set `self.AttackIndex` 3)
          (goto _label_5 :!via `Reset`))))))

(event `Stop Combo`
  ; Combo system
  ;; Stop Combo/Attack
  (set `self.isAttacking` false)
  (set `self.AttackIndex` 0))

(fn `Attack`
  (returns (animationDuration :type "Float (double-precision)"))
  (`self.Sword Attack combo call from BT`)
  (return 0.4))

(fn `BackFatal`
  (returns (refLocation :type "Vector Structure") (fatalRotation :type "Rotator Structure"))
  (`self.PlayAnimMontage` "/Game/Characters/RpgGame/Animation/Fatal/AS_OneHand_Up_Fatal_Hit_1_Montage.AS_OneHand_Up_Fatal_Hit_1_Montage")
  (return (`SceneComponent.K2_GetComponentLocation` (`self.ref location`)) (`KismetMathLibrary.MakeRotator` (.roll (`self.K2_GetActorRotation`)) (.pitch (`self.K2_GetActorRotation`)) (+ (.yaw (`self.K2_GetActorRotation`)) 30.0))))

(fn `UserConstructionScript`)