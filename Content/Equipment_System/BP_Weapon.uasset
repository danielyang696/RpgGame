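; BP_Weapon is an equipment-system weapon actor whose mesh comes from item data.
; The construction script looks up the ItemData row in its data table and, when found, applies that row's static mesh to the StaticMesh component.
; On BeginPlay it hides itself in game if IsHidden is set, and the ShowItem event clears the flag and makes it visible again.
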(event `self.ReceiveBeginPlay`
  (if (`self.IsHidden`)
    (`self.SetActorHiddenInGame` true)))

(event `/Game/Buleprints/Remiu/BPI_Show_Item.Show Item`
  (set `self.IsHidden` false)
  (`self.SetActorHiddenInGame` false))

(fn `UserConstructionScript`
  (bind _itemdata (`self.itemData`))
  (bind _returnvalue (`|GetDataTableRow` (break `DataTableRowHandle` (break `/Game/Equipment_System/S_Slot` _itemdata)) (`.RowName` (break `DataTableRowHandle` (break `/Game/Equipment_System/S_Slot` _itemdata))))
    (:`then`
      (`StaticMeshComponent.SetStaticMesh` (`self.StaticMesh`) (`.StaticMesh_9_0B455836405DB275D772E78FBDFB0834` (break `/Game/Equipment_System/S_Weapon` _returnvalue))))))