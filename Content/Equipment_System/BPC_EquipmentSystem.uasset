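; Player component for BP_ThirdPersonCharacter that handles weapon pickup and the equipment menu.
; Interact sphere-traces forward from the follow camera, stores a hit BP_Weapon's ItemData in WeaponSlots and destroys the actor.
; The menu input toggles a lazily created WB_Equipment, switching cursor and input mode, and sets the character's HasSword false while open, true on close.
; A debug key prints stored item row names.
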(event Input|EnhancedActionEvents|EnhancedInputActionIA_Interact
  (params (ActionValue :type Boolean) (ElapsedSeconds :type Float%20%28double-precision%29) (TriggeredSeconds :type Float%20%28double-precision%29) (InputAction :type Input%20Action%20Object%20Reference :default "/Game/Input/Actions/IA_Interact.IA_Interact"))
  (bind _follow_camera (Variables|Default|GetFollow%20Camera))
  (bind _returnvalue (Transformation|GetWorldLocation _follow_camera))
  ;[0.15 0.15 0.15 0.5] Pick Trace
  (:Started
    (bind (_outhit _returnvalue_2) (Collision|SphereTraceForObjects _returnvalue (+ _returnvalue (* (Math|Vector|GetForwardVector (Transformation|GetWorldRotation _follow_camera)) 1e+03)) 1e+02 (Utilities|Array|MakeArray "ObjectTypeQuery2") false 0 "None"))
    (if _returnvalue_2
      (bind _asbp_weapon (Utilities|Casting|CastToBP_Weapon (.HitActor (Collision|BreakHitResult _outhit))))
      (CallFunction|AddWeapon (Variables|/Game/Equipment_System/BP_Weapon.BP_Weapon_C|GetitemData _asbp_weapon))
      (Actor|DestroyActor _asbp_weapon))))

(event Input|EnhancedActionEvents|EnhancedInputActionIA_EquipmentMenu
  (params (ActionValue :type Boolean) (ElapsedSeconds :type Float%20%28double-precision%29) (TriggeredSeconds :type Float%20%28double-precision%29) (InputAction :type Input%20Action%20Object%20Reference :default "/Game/Input/Actions/IA_EquipmentMenu.IA_EquipmentMenu"))
  (bind _returnvalue (Game|GetPlayerController 0))
  (bind _characterbp (Variables|Default|GetCharacterBP))
  (:Started
    (if (not (Variables|Default|GetisPanelOpen))
      ;[0.15 0.15 0.15 0.5] Equipment menu panel
      (Variables|/Game/ThirdPerson/Blueprints/BP_ThirdPersonCharacter.BP_ThirdPersonCharacter_C|SethasSword _characterbp false)
      (bind _wb_equipment (Variables|Default|GetWB_Equipment)
        (:then
          (Widget|SetVisibility _wb_equipment "Visible"))
        (:else
          (bind _returnvalue_2 (UserInterface|CreateWidget "/Game/Equipment_System/UI/WB_Equipment.WB_Equipment_C"))
          (bind _output_get (Variables|Default|SetWB_Equipment _returnvalue_2))
          (UserInterface|Viewport|AddtoViewport _output_get 0)))
      (Variables|Default|SetisPanelOpen true)
      (Variables|/Script/Engine.PlayerController|SetbShowMouseCursor _returnvalue true)
      (Input|SetInputModeGameandUI _returnvalue (Variables|Default|GetWB_Equipment) "DoNotLock" true false)
      (else
        (Variables|/Game/ThirdPerson/Blueprints/BP_ThirdPersonCharacter.BP_ThirdPersonCharacter_C|SethasSword _characterbp true)
        (Variables|Default|GetWB_Equipment
          (:then
            (Widget|SetVisibility (Variables|Default|GetWB_Equipment) "Hidden")
            (Variables|Default|SetisPanelOpen false)
            (Variables|/Script/Engine.PlayerController|SetbShowMouseCursor _returnvalue false)
            (Input|SetInputModeGameOnly _returnvalue false))
          (:else))))))

(event EventBeginPlay
  (bind _asbp_third_person_character (Utilities|Casting|CastToBP_ThirdPersonCharacter (Components|GetOwner)))
  (Variables|Default|SetFollow%20Camera (Variables|/Game/ThirdPerson/Blueprints/BP_ThirdPersonCharacter.BP_ThirdPersonCharacter_C|GetFollowCamera _asbp_third_person_character))
  (Variables|Default|SetBPC%20Attack%20System (Variables|/Game/ThirdPerson/Blueprints/BP_ThirdPersonCharacter.BP_ThirdPersonCharacter_C|GetBPC_AttackSystem _asbp_third_person_character))
  (Variables|Default|SetCharacterBP _asbp_third_person_character))

(event EventTick
  (params (DeltaSeconds :type Float%20%28single-precision%29)))

(event Input|KeyboardEvents|DebugKeyH
  (params (Key :type Key%20Structure :default "None") (ActionValue :type Input%20Action%20Value%20Structure))
  ;[0.15 0.15 0.15 0.5] Pick Trace
  (:Pressed
    (for _array_element (Variables|Default|GetweaponSlots)
      (Development|PrintString (Utilities|String|ToString(Name) (.rowname (.item _array_element)))))))

(fn AddWeapon
  (params (newItem :type S%20Slot%20Structure))
  (Utilities|Array|Add (Variables|Default|GetweaponSlots) newItem))