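; BP_AIController_Boss is the boss AI controller, running the boss behavior tree and managing the boss health bar on screen.
; BeginPlay starts BT_AI_Boss, whose chase-target task calls ActivateBossFight to create the health bar widget if the boss has health left and none exists.
; Tick feeds the health ratio into the bar while it exists.
; DeactivateBossFight removes the widget and clears its reference.
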(event `self.ReceiveBeginPlay`
  (`self.RunBehaviorTree` "/Game/AI/Boss/BT_AI_Boss.BT_AI_Boss"))

(event `self.ReceiveTick`
  (params (DeltaSeconds :type "Float (single-precision)"))
  (bind _bosshealthbarwidget (`self.bossHealthBarWidget`)
    (:`then`
      (`ProgressBar.SetPercent` (`/Game/UI/WB_BossHealthbar.HealthBar` _bosshealthbarwidget) (/ (`self.currentHealth`) (`self.maxHealth`))))
    (:`else`)))

(event `Activate Boss Fight`
  ; this event called by  BT_Task_ChaseTarget
  (if (> (`self.currentHealth`) 0.0)
    (`self.bossHealthBarWidget`
      (:`then`)
      (:`else`
        (bind _returnvalue (`|CreateWidget` "/Game/UI/WB_BossHealthbar.WB_BossHealthbar_C"))
        (bind _output_get (set `self.bossHealthBarWidget` _returnvalue))
        (`UserWidget.AddToViewport` _output_get 0)))))

(event `Deactivate Boss Fight`
  (`self.bossHealthBarWidget`
    (:`then`
      (`Widget.RemoveFromParent` (`self.bossHealthBarWidget`))
      (set `self.bossHealthBarWidget` null))
    (:`else`)))

(fn `UserConstructionScript`
  (`parent.UserConstructionScript`))