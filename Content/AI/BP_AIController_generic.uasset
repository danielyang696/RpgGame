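; Generic AI controller that runs BT_AI and feeds it sight and hearing perception through the Blackboard.
; Successful sight stores the Target Actor, while hearing stores InvestigationLocation.
; Lost sight, or any non-sight stimulus including hearing, clears the target.
; On that clear, the controller casts itself to BP_AIController_Boss and deactivates the boss fight if the cast succeeds.
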(event `self.ReceiveBeginPlay`
  (`self.RunBehaviorTree` "/Game/AI/BT_AI.BT_AI"))

(event `self.AIPerception.OnTargetPerceptionUpdated`
  (params (Actor :type "Actor Object Reference") (Stimulus :type "AIStimulus Structure"))
  ; Detect and chase target
  (`self.SightDetection` Actor Stimulus)
  (`self.HearingDetection` Actor Stimulus))

(fn `HearingDetection`
  (params (actor :type "Actor Object Reference") (`stimulus ` :type "AIStimulus Structure"))
  (bind _returnvalue (`AIPerceptionSystem.GetSenseClassForStimulus` `stimulus `))
  (if (== _returnvalue "/Script/AIModule.AISense_Hearing")
    (`BlackboardComponent.SetValueAsVector` (`AIBlueprintHelperLibrary.GetBlackboard` null) "InvestigationLocation" (`.StimulusLocation` (break `AIStimulus` `stimulus `)))))

(fn `SightDetection`
  (params (actor :type "Actor Object Reference") (`stimulus ` :type "AIStimulus Structure"))
  (bind _returnvalue (`AIPerceptionSystem.GetSenseClassForStimulus` `stimulus `))
  (if (== _returnvalue "/Script/AIModule.AISense_Sight")
    (if (`.bSuccessfullySensed` (break `AIStimulus` `stimulus `))
      (`BlackboardComponent.SetValueAsObject` (`AIBlueprintHelperLibrary.GetBlackboard` null) "Target Actor" actor)
      (else
        (`BlackboardComponent.SetValueAsObject` (`AIBlueprintHelperLibrary.GetBlackboard` null) "Target Actor" null :!label _label)
        (bind _asbp_aicontroller_boss (cast `/Game/AI/Boss/BP_AIController_Boss` self))
        (`/Game/AI/Boss/BP_AIController_Boss.Deactivate Boss Fight` _asbp_aicontroller_boss)))
    (else
      (goto _label))))

(fn `UserConstructionScript`)